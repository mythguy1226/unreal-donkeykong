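; BP_BombExplosion is a bomb explosion actor that restarts the level if the player is caught in its blast.
; On BeginPlay it pauses the game, delays for the length of its flipbook sprite, then unpauses.
; It then runs a sphere trace on the Camera channel around itself, reopens the current level for a BP_Player hit, and destroys itself.
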(event EventBeginPlay
  (bind _returnvalue (Transformation|GetActorLocation))
  (Game|SetGamePaused true)
  (Utilities|FlowControl|Delay (Class|PaperFlipbookComponent|GetFlipbookLength (Variables|Default|GetSprite)))
  (Game|SetGamePaused false)
  (bind _outhits (Collision|MultiSphereTraceByChannel _returnvalue _returnvalue 1e+02 "TraceTypeQuery2" false 0 "None"))
  (for _array_element _outhits
    (Utilities|Casting|CastToBP_Player (.HitActor (Collision|BreakHitResult _array_element)))
    (bind _returnvalue_2 (Game|GetCurrentLevelName true))
    (Game|OpenLevel(byName) (Utilities|String|StringToName _returnvalue_2)))
  (Actor|DestroyActor))

(fn ConstructionScript
  (|CallParentFunction))