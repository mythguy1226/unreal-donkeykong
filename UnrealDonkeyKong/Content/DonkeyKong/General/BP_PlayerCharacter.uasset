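; BP_PlayerCharacter is the player-controlled character for a Donkey Kong game, providing horizontal movement and jumping.
; On BeginPlay it registers the IMC_PlayerInputMap mapping context with the controller's Enhanced Input subsystem.
; IA_Move feeds its clamped X value into movement along the fixed world right (Y) axis, independent of character or camera rotation.
; IA_Jump triggers the built-in Character jump.
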(event Input|EnhancedActionEvents|EnhancedInputActionIA_Move
  (params (ActionValue :type Vector%202D%20Structure) (ElapsedSeconds :type Float%20%28double-precision%29) (TriggeredSeconds :type Float%20%28double-precision%29) (InputAction :type Input%20Action%20Object%20Reference :default "/Game/DonkeyKong/Input/IA_Move.IA_Move"))
  (Pawn|Input|AddMovementInput (Math|Vector|GetRightVector "0, 0, 0") (Math|Float|Clamp(Float) (.x ActionValue) -1.0) false))

(event Input|EnhancedActionEvents|EnhancedInputActionIA_Jump
  (params (ActionValue :type Boolean) (ElapsedSeconds :type Float%20%28double-precision%29) (TriggeredSeconds :type Float%20%28double-precision%29) (InputAction :type Input%20Action%20Object%20Reference :default "/Game/DonkeyKong/Input/IA_Jump.IA_Jump"))
  (Character|Jump))

(event EventBeginPlay
  (bind _asplayer_controller (Utilities|Casting|CastToPlayerController (Pawn|GetController)))
  (Utilities|IsValid (PlayerController|LocalPlayerSubsystems|GetEnhancedInputLocalPlayerSubsystem _asplayer_controller)
    (:Is%20Valid
      (Input|AddMappingContext (PlayerController|LocalPlayerSubsystems|GetEnhancedInputLocalPlayerSubsystem _asplayer_controller) "/Game/DonkeyKong/Input/IMC_PlayerInputMap.IMC_PlayerInputMap" 0 "(bIgnoreAllPressedKeysUntilRelease=True,bForceImmediately=False,bNotifyUserSettings=False)"))))

(fn ConstructionScript)