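; Player character for a Donkey Kong-style game, with sideways movement, jumping and climbing.
; Enhanced Input, mapped on BeginPlay, drives jump and single-axis movement, which is blocked while Climbing and yaws the sprite toward velocity.
; Hard-coded W and S presses, gated by CanClimb, switch to Flying mode, add one vertical input and set Climbing.
; This graph never sets CanClimb, clears Climbing or restores walking.
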(event Input|EnhancedActionEvents|EnhancedInputActionIA_Move
  (params (ActionValue :type Vector%202D%20Structure) (ElapsedSeconds :type Float%20%28double-precision%29) (TriggeredSeconds :type Float%20%28double-precision%29) (InputAction :type Input%20Action%20Object%20Reference :default "/Game/DonkeyKong/Input/IA_Move.IA_Move"))
  (bind _returnvalue (Transformation|GetActorLocation))
  (if (not (Variables|Default|GetbClimbing))
    (Pawn|Input|AddMovementInput (* (Math|Vector|GetForwardVector "0, 0, 0") -1.0) (Math|Float|Clamp(Float) (.x ActionValue) -1.0) false)
    (Transformation|SetWorldRotation (Variables|Default|GetSprite) (Math|Rotator|MakeRotator 0.0 0.0 (.yaw (Math|Rotator|FindLookatRotation _returnvalue (+ _returnvalue (Math|Vector|Normalize (Transformation|GetVelocity)))))) false false)))

(event Input|EnhancedActionEvents|EnhancedInputActionIA_Jump
  (params (ActionValue :type Boolean) (ElapsedSeconds :type Float%20%28double-precision%29) (TriggeredSeconds :type Float%20%28double-precision%29) (InputAction :type Input%20Action%20Object%20Reference :default "/Game/DonkeyKong/Input/IA_Jump.IA_Jump"))
  (Character|Jump))

(event EventBeginPlay
  (bind _asplayer_controller (Utilities|Casting|CastToPlayerController (Pawn|GetController)))
  (Utilities|IsValid (PlayerController|LocalPlayerSubsystems|GetEnhancedInputLocalPlayerSubsystem _asplayer_controller)
    (:Is%20Valid
      (Input|AddMappingContext (PlayerController|LocalPlayerSubsystems|GetEnhancedInputLocalPlayerSubsystem _asplayer_controller) "/Game/DonkeyKong/Input/IMC_PlayerInputMap.IMC_PlayerInputMap" 0 "(bIgnoreAllPressedKeysUntilRelease=True,bForceImmediately=False,bNotifyUserSettings=False)"))))

(event Input|KeyboardEvents|W
  (params (Key :type Key%20Structure :default "None"))
  (:Pressed
    (if (Variables|Default|GetbCanClimb)
      (Pawn|Components|CharacterMovement|SetMovementMode (Variables|Character|GetCharacterMovement) "MOVE_Flying" 0)
      (Pawn|Input|AddMovementInput "0.000000,0.000000,1.000000" 1.0 true)
      (Variables|Default|SetbClimbing true))))

(event Input|KeyboardEvents|S
  (params (Key :type Key%20Structure :default "None"))
  (:Pressed
    (if (Variables|Default|GetbCanClimb)
      (Pawn|Components|CharacterMovement|SetMovementMode (Variables|Character|GetCharacterMovement) "MOVE_Flying" 0)
      (Pawn|Input|AddMovementInput "0.000000,0.000000,-1.000000" 1.0 true)
      (Variables|Default|SetbClimbing true))))

(fn ConstructionScript)