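; BP_PhaseBlock is a Donkey Kong block that lets pawns pass through while the player is climbing and is solid otherwise.
; On BeginPlay it caches the player character as a BP_Player reference.
; Every Tick, after running the parent logic, it reads the player's Climbing flag and switches the Box's Pawn collision response between Overlap and Block.
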(event EventTick
  (params (DeltaSeconds :type Float%20%28single-precision%29))
  (|CallParentFunction DeltaSeconds)
  (if (Variables|/Game/DonkeyKong/General/BP_Player.BP_Player_C|GetbClimbing (Variables|Default|GetPlayerRef))
    (Collision|SetCollisionResponsetoChannel (Variables|Default|GetBox) "ECC_Pawn" "ECR_Overlap")
    (else
      (Collision|SetCollisionResponsetoChannel (Variables|Default|GetBox) "ECC_Pawn" "ECR_Block"))))

(event EventBeginPlay
  (bind _asbp_player (Utilities|Casting|CastToBP_Player (Game|GetPlayerCharacter 0)))
  (Variables|Default|SetPlayerRef _asbp_player))

(fn ConstructionScript
  (|CallParentFunction))