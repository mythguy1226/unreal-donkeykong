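; BP_Ladder is a Donkey Kong ladder block that controls when the player can climb.
; Overlapping its box on a Climbable ladder lets a player without the mallet climb and stores the ladder's location on them.
; Leaving the box resets climb state and restores walking, always on Top pieces, but on other pieces only if the player is not climbing.
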(event OnComponentBeginOverlap(Box)
  (params (OverlappedComponent :type Primitive%20Component%20Object%20Reference) (OtherActor :type Actor%20Object%20Reference) (OtherComp :type Primitive%20Component%20Object%20Reference) (OtherBodyIndex :type Integer) (bFromSweep :type Boolean) (SweepResult :type Hit%20Result%20Structure%20%28by%20ref%29))
  (if (Variables|Default|GetbClimbable)
    (bind _asbp_player (Utilities|Casting|CastToBP_Player OtherActor))
    (if (not (Variables|/Game/DonkeyKong/General/BP_Player.BP_Player_C|GetbUsingMallet _asbp_player))
      (Variables|/Game/DonkeyKong/General/BP_Player.BP_Player_C|SetbCanClimb _asbp_player true)
      (Variables|/Game/DonkeyKong/General/BP_Player.BP_Player_C|SetCurrentLadderLoc _asbp_player (Transformation|GetActorLocation)))))

(event OnComponentEndOverlap(Box)
  (params (OverlappedComponent :type Primitive%20Component%20Object%20Reference) (OtherActor :type Actor%20Object%20Reference) (OtherComp :type Primitive%20Component%20Object%20Reference) (OtherBodyIndex :type Integer))
  (if (Variables|Default|GetbTop)
    (bind _asbp_player (Utilities|Casting|CastToBP_Player OtherActor))
    (Variables|/Game/DonkeyKong/General/BP_Player.BP_Player_C|SetbClimbing _asbp_player false)
    (Variables|/Game/DonkeyKong/General/BP_Player.BP_Player_C|SetbCanClimb _asbp_player false)
    (Pawn|Components|CharacterMovement|SetMovementMode (Variables|/Script/Engine.Character|GetCharacterMovement _asbp_player) "MOVE_Walking" 0)
    (else
      (bind _asbp_player_2 (Utilities|Casting|CastToBP_Player OtherActor))
      (if (not (Variables|/Game/DonkeyKong/General/BP_Player.BP_Player_C|GetbClimbing _asbp_player_2))
        (Variables|/Game/DonkeyKong/General/BP_Player.BP_Player_C|SetbClimbing _asbp_player_2 false)
        (Variables|/Game/DonkeyKong/General/BP_Player.BP_Player_C|SetbCanClimb _asbp_player_2 false)
        (Pawn|Components|CharacterMovement|SetMovementMode (Variables|/Script/Engine.Character|GetCharacterMovement _asbp_player_2) "MOVE_Walking" 0)))))

(fn ConstructionScript
  (|CallParentFunction))