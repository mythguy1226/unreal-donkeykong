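; Donkey Kong enemy Blueprint that repeatedly throws barrels.
; On BeginPlay it plays a throw animation override on the animation component and waits for its completion callback.
; On completion it spawns a BP_Barrel at the BarrelSpawnPoint, gives it a default controller, and sets a cooldown timer that restarts the cycle.
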(event Custom|SpawnBarrel
  (|PlayAnimationOverridewithCallbacks (Variables|/Script/PaperZD.PaperZDAnimationComponent|GetAnimInstance (Variables|Default|GetAnimationComponent)) "/Game/DonkeyKong/AI/DonkeyKong/AnimSequences/AS_ThrowBarrel.AS_ThrowBarrel" "DefaultSlot" 1.0 0.0
    (:OnCompleted
      (CallFunction|ThrowBarrel)
      (Utilities|Time|SetTimerbyEvent (delegate Custom|SpawnBarrel) (Variables|Default|GetThrowCooldown)))))

(event EventBeginPlay
  (CallFunction|SpawnBarrel))

(fn ConstructionScript)

(fn ThrowBarrel
  (bind _returnvalue (Game|SpawnActorfromClass "/Game/DonkeyKong/AI/Barrels/BP_Barrel.BP_Barrel_C" (Math|Transform|MakeTransform (Transformation|GetWorldLocation (Variables|Default|GetBarrelSpawnPoint))) "Undefined" "MultiplyWithRoot" 0 0))
  (Pawn|SpawnDefaultController _returnvalue))