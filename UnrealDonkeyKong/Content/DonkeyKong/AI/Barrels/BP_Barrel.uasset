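; BP_Barrel is a rolling barrel hazard in the Donkey Kong game that restarts the level when it hits the player.
; Every tick it applies forced movement input along its reversed forward vector, scaled by Speed.
; Capsule hits drive the rest: a BlockingVolume flips the sign of Speed to reverse direction, and BP_Player triggers a reload of the current level by name.
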(event OnComponentHit(CapsuleComponent)
  (params (HitComponent :type Primitive%20Component%20Object%20Reference) (OtherActor :type Actor%20Object%20Reference) (OtherComp :type Primitive%20Component%20Object%20Reference) (NormalImpulse :type Vector :default "0, 0, 0") (Hit :type Hit%20Result%20Structure%20%28by%20ref%29))
  (Utilities|FlowControl|Sequence
    (:then_0
      (Utilities|Casting|CastToBlockingVolume OtherActor)
      (Variables|Default|SetSpeed (* (Variables|Default|GetSpeed) -1.0)))
    (:then_1
      (Utilities|Casting|CastToBP_Player OtherActor)
      (bind _returnvalue (Game|GetCurrentLevelName true))
      (Game|OpenLevel(byName) (Utilities|String|StringToName _returnvalue)))))

(event EventTick
  (params (DeltaSeconds :type Float%20%28single-precision%29))
  (Pawn|Input|AddMovementInput (* (Transformation|GetActorForwardVector) -1.0) (Variables|Default|GetSpeed) true))

(fn ConstructionScript)